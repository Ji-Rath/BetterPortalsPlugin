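; BP_PortalManager is the manager actor that initializes the game's portals and their post-process effect.
; Shortly after BeginPlay, a brief delay precedes a SetupPortals call on its PortalManager.
; It then replaces the PostProcess settings with a single full-weight blendable built from the manager's dynamic portal post-process material.
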(event `self.ReceiveBeginPlay`
  (`parent.ReceiveBeginPlay`)
  (`KismetSystemLibrary.Delay` 1.5)
  (`PortalManagerComponent.SetupPortals` (`self.PortalManager`))
  (set `PostProcessComponent.Settings` (make `PostProcessSettings` :`WeightedBlendables` (make `WeightedBlendables` (`|MakeArray` (make `WeightedBlendable` 1.0 (`PortalManagerComponent.PortalPPDynamic` (`self.PortalManager`)))))) (`self.PostProcess`)))

(fn `UserConstructionScript`)