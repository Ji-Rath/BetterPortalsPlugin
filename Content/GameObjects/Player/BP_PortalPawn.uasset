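; BP_PortalPawn is the player pawn, handling physics velocity limiting, HUD setup and interaction input.
; BeginPlay creates the BP_PlayerWidget, adds it to the viewport and sets game-only input.
; Each tick, LimitVelocity clamps the simulating capsule's linear velocity to PlayerMaxVel to avoid destruction-related crashes.
; E press and release pass true or false to InteractAction, intended for physics objects on the Interactable collision channel.
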(event `self.ReceiveTick`
  (params (DeltaSeconds :type "Float (single-precision)"))
  ;[0.1881 1 0] Limit player velocity to avoid destruction crashes.
  (`parent.ReceiveTick` DeltaSeconds)
  (`self.LimitVelocity`))

(event `self.ReceiveBeginPlay`
  ;[1 0.02512 0] Add Widget to Viewport...
  (`parent.ReceiveBeginPlay`)
  (bind _returnvalue (`|CreateWidget` "/BetterPortals/GameObjects/Player/UI/BP_PlayerWidget.BP_PlayerWidget_C"))
  (bind _output_get (set `self.UserInterface` _returnvalue))
  (`UserWidget.AddToViewport` _output_get 0)
  (`WidgetBlueprintLibrary.SetInputMode_GameOnly` (`GameplayStatics.GetPlayerController` 0)))

(event `Key|E`
  (params (Key :type "Key Structure"))
  ;[0 0.9335 1] Pass input to interact functions. NOTE: Any physics object with collision object channel Interactable
  (:`Pressed`
    (`self.InteractAction` true))
  (:`Released`
    (`self.InteractAction` false)))

(fn `LimitVelocity`
  (bind _playermaxvel (`self.playerMaxVel`))
  (if (`SceneComponent.IsSimulatingPhysics` (`self.playerCapsule`) "None")
    (bind _returnvalue (`PrimitiveComponent.GetPhysicsLinearVelocity` (`self.playerCapsule`) "None"))
    (if (> (`KismetMathLibrary.VSize` _returnvalue) _playermaxvel)
      (`PrimitiveComponent.SetPhysicsLinearVelocity` (`self.playerCapsule`) (`KismetMathLibrary.ClampVectorSize` _returnvalue 0.0 _playermaxvel) false "None"))))

(fn `UserConstructionScript`)